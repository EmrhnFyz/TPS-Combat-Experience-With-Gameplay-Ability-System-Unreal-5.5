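; Survival game mode Blueprint that shows wave announcement UI as the game mode's state changes.
; On BeginPlay it binds to the state-changed delegate and switches on the state to spawn countdown or plain text wave widgets through two helper functions.
; The final wave also sets the enemy spawn delay and shows a delayed "Last Wave" message, while all-waves-done and player-death states only print strings.
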(event Custom|OnSurvivalGameModeStateChanged_Event
  (params (CurrentState :type ETPSCombatSurvivalGameModeState%20Enum :default "WaitSpawnNewWave"))
  (switch Utilities|FlowControl|Switch|SwitchonETPSCombatSurvivalGameModeState CurrentState
    (:WaitSpawnNewWave
      (CallFunction|CreateWaveWidgetwithCountDown "New Wave Coming In" (Variables|Default|GetSpawnNewWaveWaitTime)))
    (:SpawningNewWave
      (CallFunction|CreateWaveWidgetNoCountDown (Utilities|Text|FormatText "Wave {CurrentWaveCount}" (Variables|Default|GetCurrentWaveCount)))
      (if (== (Variables|Default|GetTotalWavesToSpawn) (Variables|Default|GetCurrentWaveCount))
        (Variables|Default|SetSpawnEnemiesDelayTime 4.0)
        (Utilities|FlowControl|Delay 2.0)
        (CallFunction|CreateWaveWidgetNoCountDown "Last Wave")))
    (:WaveCompleted
      (CallFunction|CreateWaveWidgetwithCountDown (Utilities|Text|FormatText "Wave {CurrentWaveCount} Completed" (Variables|Default|GetCurrentWaveCount)) (Variables|Default|GetWaveCompletedWaitTime)))
    (:AllWavesDone
      (Development|PrintString "All Waves  completed"))
    (:PlayerDied
      (Development|PrintString "GIT GUD" true true "(R=1.000000,G=0.000000,B=0.062274,A=1.000000)"))))

(event EventBeginPlay
  (EventDispatchers|AssignOnSurvivalGameModeStateChanged (delegate Custom|OnSurvivalGameModeStateChanged_Event)))

(event EventTick
  (params (DeltaSeconds :type Float%20%28single-precision%29)))

(fn ConstructionScript)

(fn CreateWaveWidgetwithCountDown
  (params (TextContentToDisplay :type Text) (InTotalCountDownTime :type Float%20%28double-precision%29))
  (bind _returnvalue (UserInterface|CreateWidget "/Game/Widgets/GameModeWidgets/WBP_WaveTextWithCounter.WBP_WaveTextWithCounter_C"))
  (UserInterface|Viewport|AddtoViewport _returnvalue 0)
  (Rendering|Components|TextRender|SetText (Variables|/Game/Widgets/GameModeWidgets/WBP_WaveTextWithCounter.WBP_WaveTextWithCounter_C|GettTextBlock_WaveText _returnvalue) TextContentToDisplay)
  (Default|StartCountDownEvent _returnvalue InTotalCountDownTime))

(fn CreateWaveWidgetNoCountDown
  (params (TextContentToDisplay :type Text))
  (bind _returnvalue (UserInterface|CreateWidget "/Game/Widgets/GameModeWidgets/WBP_WaveTextNoCounter.WBP_WaveTextNoCounter_C"))
  (UserInterface|Viewport|AddtoViewport _returnvalue 0)
  (Rendering|Components|TextRender|SetText (Variables|/Game/Widgets/GameModeWidgets/WBP_WaveTextNoCounter.WBP_WaveTextNoCounter_C|GettTextBlock_WaveText _returnvalue) TextContentToDisplay))