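; Base projectile Blueprint that handles cosmetic sound and effects for projectiles.
; On BeginPlay it plays a cast sound, attaches a flying sound that stops with the projectile, and spawns a forward-facing muzzle effect.
; OnSpawnProjectileHitFX plays the impact sound at the hit location, but its impact effect spawn is disconnected and never runs.
; Each asset is validity-checked before use, and movement and hit detection are absent from these graphs.
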(event EventBeginPlay
  (Utilities|FlowControl|Sequence
    (:then_0
      (bind _projectile_cast_sound (Variables|Default|GetProjectile%20Cast%20Sound)
        (:then
          (Audio|PlaySoundatLocation _projectile_cast_sound (Transformation|GetActorLocation) "0, 0, 0" 1.0 1.0 0.0 0 0 0 0))
        (:else)))
    (:then_1
      (bind _projectile_flying_sound (Variables|Default|GetProjectile%20Flying%20Sound)
        (:then
          (Audio|SpawnSoundAttached _projectile_flying_sound (Variables|Transformation|GetRootComponent) "None" "0, 0, 0" "0, 0, 0" "KeepRelativeOffset" true 1.0 1.0 0.0 0 0))
        (:else)))
    (:then_2
      (bind _projectile_muzzle_fx (Variables|Default|GetProjectile%20Muzzle%20FX)
        (:then
          (Niagara|SpawnSystematLocation _projectile_muzzle_fx (Transformation|GetActorLocation) (Math|Conversions|RotationFromXVector (Transformation|GetActorForwardVector))))
        (:else)))))

(event EventOnSpawnProjectileHitFX
  (params (HitLocation :type Vector%20%28by%20ref%29 :default "0, 0, 0"))
  (Utilities|FlowControl|Sequence
    (:then_0
      (bind _projectile_impact_sound (Variables|Default|GetProjectile%20Impact%20Sound)
        (:then
          (Audio|PlaySoundatLocation _projectile_impact_sound HitLocation "0, 0, 0" 1.0 1.0 0.0 0 0 0 0))
        (:else)))
    (:then_1
      (bind _projectile_impact_fx (Variables|Default|GetProjectile%20Impact%20FX)
        (:then)
        (:else)))))

(fn ConstructionScript)